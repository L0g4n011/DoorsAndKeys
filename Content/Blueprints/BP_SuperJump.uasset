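; BP_SuperJump is a pickup item that attaches to the hand_r socket and launches the third-person character upward.
; Pickup disables PowerUp collision and prints a message still naming it "Machine Gun"; Drop only detaches it.
; UsePrimary enables physics on the character's capsule and applies a large upward impulse.
; UseSecondary switches that physics off to "regain control", with both finding the character through GetActorOfClass.
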(event EventBeginPlay)

(event EventPickup
  (params (SkeletalMesh :type Skeletal%20Mesh%20Component%20Object%20Reference))
  ;[0.294 1 0.2514] Pickup Function
  (Development|PrintText (Utilities|Text|FormatText "{name} is getting picked up." (Utilities|String|MakeLiteralString "Machine Gun")) true true "(R=1.000000,G=0.000000,B=0.800960,A=1.000000)")
  (Transformation|AttachComponentToComponent SkeletalMesh "hand_r" "SnapToTarget" "SnapToTarget" "SnapToTarget" true)
  (Collision|SetCollisionEnabled (Variables|Default|GetPowerUp) "NoCollision"))

(event EventUsePrimary
  (Development|PrintText "Bounce")
  (bind _returnvalue (Actor|GetActorOfClass "/Game/ThirdPerson/Blueprints/BP_ThirdPersonCharacter.BP_ThirdPersonCharacter_C"))
  (Physics|SetSimulatePhysics (Variables|/Script/Engine.Character|GetCapsuleComponent _returnvalue) true)
  (Physics|AddImpulse (Variables|/Script/Engine.Character|GetCapsuleComponent _returnvalue) "0.000000,0.000000,1000000.000000" "None" false))

(event EventUseSecondary
  (Development|PrintText "Regain control")
  (bind _returnvalue (Actor|GetActorOfClass "/Game/ThirdPerson/Blueprints/BP_ThirdPersonCharacter.BP_ThirdPersonCharacter_C"))
  (Physics|SetSimulatePhysics (Variables|/Script/Engine.Character|GetCapsuleComponent _returnvalue) false))

(event EventDrop
  (params (SkeletalMesh :type Skeletal%20Mesh%20Component%20Object%20Reference))
  (Transformation|DetachFromActor "KeepRelative" "KeepRelative" "KeepRelative"))

(fn ConstructionScript)