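; BP_LoopsAndLists is a demo Blueprint of loops and lists that prints debug messages.
; DelayLoop prints and increments a counter, waits briefly, calls PrintColors, then calls itself to repeat indefinitely.
; PrintColors iterates over an inline array of colors, printing a string in each.
; BeginPlay is empty and the startup chain calling DelayLoop is disconnected, so nothing in this graph starts the loop.
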(event Custom|Delay%20Loop
  (Development|PrintString (Utilities|String|Append "Starting Delay Loop # " (Utilities|String|ToString(Integer) (Variables|Default|GetDelayLoopCounter))))
  (Math|Integer|IncrementInt (Variables|Default|GetDelayLoopCounter)
    (:%20%20
      (Utilities|FlowControl|Delay 0.2)
      (CallFunction|PrintColors)
      (CallFunction|DelayLoop))))

(event Custom|Print%20Colors
  (for _array_element (Utilities|Array|MakeArray "(R=1.000000,G=0.145093,B=0.256207,A=1.000000)" "(R=0.000000,G=0.393597,B=1.000000,A=1.000000)" "(R=0.927257,G=1.000000,B=0.080056,A=1.000000)" "(R=0.294010,G=1.000000,B=0.251361,A=1.000000)" "(R=0.156495,G=0.896102,B=1.000000,A=1.000000)")
    (Development|PrintString "Hello" true true _array_element)))

(event EventBeginPlay)

(event Collision|EventActorBeginOverlap
  (params (OtherActor :type Actor%20Object%20Reference)))

(event EventTick
  (params (DeltaSeconds :type Float%20%28single-precision%29)))

(fn ConstructionScript)