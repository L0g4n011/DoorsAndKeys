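; Enemy spawner that places one BP_AiMoveTo character at every BP_EnemySpawnPoint in the level when play begins.
; On BeginPlay it gathers all spawn point actors and spawns at each one's transform.
; Each spawn gets a randomly picked skeletal mesh and first-slot material for visual variety.
; A random name is printed to announce each spawn but is not stored on the character.
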(event EventBeginPlay
  (Development|PrintString "Enemy Spawner is Active")
  (bind _outactors (Actor|GetAllActorsOfClass "/Game/Blueprints/BP_EnemySpawnPoint.BP_EnemySpawnPoint_C"))
  (for _array_element _outactors
    (bind _returnvalue (Game|SpawnActorfromClass "/Game/AI_Blueprints/BP_AiMoveTo.BP_AiMoveTo_C" (Transformation|GetActorTransform _array_element) "Undefined" "MultiplyWithRoot" 0 0))
    (Components|SkeletalMesh|SetSkeletalMeshAsset (Variables|/Script/Engine.Character|GetMesh _returnvalue) (.OutItem (Utilities|Array|Random (Utilities|Array|MakeArray (Variables|Default|GetSkeletalMesh) "/Game/SCK_Casual01/Models/MESH_A_01.MESH_A_01" "/Game/SCK_Casual01/Models/MESH_A_03.MESH_A_03" "/Game/SCK_Casual01/Models/Premade_Characters/MESH_PC_00.MESH_PC_00"))))
    (Development|PrintString (Utilities|String|Append "Now Spawning: " (.OutItem (Utilities|Array|Random (Utilities|Array|MakeArray (Variables|Default|GetName) "Levi" "Alex" "Smith" "George")))))
    (Rendering|Material|SetMaterial (Variables|/Script/Engine.Character|GetMesh _returnvalue) 0 (.OutItem (Utilities|Array|Random (Utilities|Array|MakeArray (Variables|Default|GetMaterials) "/Game/PolygonStarter/Materials/M_Polygon_Plane_01.M_Polygon_Plane_01" "/Game/PolygonStarter/Materials/M_Polygon_Plane_02.M_Polygon_Plane_02" "/Game/PolygonStarter/Materials/M_Polygon_Plane_03.M_Polygon_Plane_03"))))))

(fn ConstructionScript)