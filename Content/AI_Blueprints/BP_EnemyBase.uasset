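; BP_EnemyBase is an enemy base Blueprint that provides attack and aggro behavior.
; Attack prints debug text, plays a ninja wheel kick montage on the mesh, and calls AttackFinished whether the montage completes or is interrupted.
; GetAggro swaps the mesh to a flat red material and sets an Aggroed flag, while LoseAggro restores the material cached at BeginPlay and clears it.
; SetSpeed is an empty stub.
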(event Custom|Attack
  (Development|PrintText "Attack")
  (Animation|Montage|PlayMontage (Variables|Character|GetMesh) "/Game/CloseCombatAnimSet/Animations/InPlace/Attacks/NinjaWheelKick_Montage.NinjaWheelKick_Montage"
    (:OnCompleted
      _)
    (:OnInterrupted
      _))
  (Default|CallAttackFinished))

(event Custom|Get%20Aggro
  (Rendering|Material|SetMaterial (Variables|Character|GetMesh) 0 "/Game/Materials/MI_FlatRed.MI_FlatRed")
  (Variables|Default|SetAggroed true))

(event Custom|Lose%20Aggro
  (Rendering|Material|SetMaterial (Variables|Character|GetMesh) 0 (Variables|Default|GetOriginalMaterial))
  (Variables|Default|SetAggroed false))

(event Custom|Set%20Speed
  (params (New%20Speed :type Float%20%28double-precision%29)))

(event EventBeginPlay
  (Variables|Default|SetOriginalMaterial (Rendering|Material|GetMaterial (Variables|Character|GetMesh) 0)))

(fn ConstructionScript)