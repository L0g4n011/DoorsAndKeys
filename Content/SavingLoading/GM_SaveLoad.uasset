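; Game Mode that saves and loads player stats and per-level state through two SaveGame objects, SG_PlayerStats and SG_LevelState.
; BeginPlay loads the fixed PlayerSave slot and applies Stamina to BP_ThirdPersonCharacter, creating a new save object if none exists.
; Level state uses the level name as its slot, and loading calls AlreadyCollected on each saved coin reference.
; Save events write the held objects as they are, with printed status messages.
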(event Custom|Load%20Player%20Stats
  (bind _returnvalue (SaveGame|DoesSaveGameExist "PlayerSave"))
  (if _returnvalue
    (bind _returnvalue_2 (SaveGame|LoadGamefromSlot "PlayerSave"))
    (bind _assg_player_stats (Utilities|Casting|CastToSG_PlayerStats _returnvalue_2))
    (Variables|Default|SetSG_PlayerStats _assg_player_stats)
    (bind _asbp_third_person_character (Utilities|Casting|CastToBP_ThirdPersonCharacter (Game|GetPlayerCharacter 0)))
    (Variables|/Game/ThirdPerson/Blueprints/BP_ThirdPersonCharacter.BP_ThirdPersonCharacter_C|SetStamina _asbp_third_person_character (Variables|/Game/SavingLoading/SG_PlayerStats.SG_PlayerStats_C|GetStamina (Variables|Default|GetSG_PlayerStats)))
    (Development|PrintText "PlayerStats has been loaded" true true "(R=1.000000,G=0.526450,B=0.000000,A=1.000000)")
    (else
      (bind _returnvalue_3 (SaveGame|CreateSaveGameObject "/Game/SavingLoading/SG_PlayerStats.SG_PlayerStats_C"))
      (Variables|Default|SetSG_PlayerStats _returnvalue_3))))

(event Custom|Save%20Player%20Stats
  (bind _returnvalue (SaveGame|SaveGametoSlot (Variables|Default|GetSG_PlayerStats) "PlayerSave"))
  (if _returnvalue
    (Development|PrintText "Player Stats Written to Save Game File" true true "(R=0.033646,G=1.000000,B=0.023452,A=1.000000)")
    (else
      (Development|PrintText "Player Stats Could not be Written to Save Game File" true true "(R=1.000000,G=0.000066,B=0.016391,A=1.000000)"))))

(event Custom|Save%20Level%20State
  (bind _returnvalue (Game|GetCurrentLevelName true))
  (bind _returnvalue_2 (SaveGame|SaveGametoSlot (Variables|Default|GetSG_LevelState) _returnvalue))
  (if _returnvalue_2
    (Development|PrintText "Level State Written to Save Game File" true true "(R=0.033647,G=1.000000,B=0.023452,A=1.000000)")
    (else
      (Development|PrintText "Player Stats Could Not Be Written to Save Game File" true true "(R=1.000000,G=0.000066,B=0.016391,A=1.000000)"))))

(event Custom|Load%20Level%20State
  (bind _returnvalue (Game|GetCurrentLevelName true))
  (bind _returnvalue_2 (SaveGame|DoesSaveGameExist _returnvalue))
  (if _returnvalue_2
    (bind _returnvalue_3 (SaveGame|LoadGamefromSlot _returnvalue))
    (bind _assg_level_state (Utilities|Casting|CastToSG_LevelState _returnvalue_3))
    (bind _output_get (Variables|Default|SetSG_LevelState _assg_level_state))
    ;[0.15 0.15 0.15 0.5] Loads the coins
    (for _array_element (Variables|/Game/SavingLoading/SG_LevelState.SG_LevelState_C|GetCollectedCoins _output_get)
      (Utilities|IsValid _array_element
        (:Is%20Valid
          (Default|AlreadyCollected _array_element))))
    (Development|PrintText "Coin State Loaded")
    (else
      (bind _returnvalue_4 (SaveGame|CreateSaveGameObject "/Game/SavingLoading/SG_LevelState.SG_LevelState_C"))
      (Variables|Default|SetSG_LevelState _returnvalue_4))))

(event EventBeginPlay
  (Development|PrintText "Loading the SaveLoad Game Mode" true true "(R=1.000000,G=0.526450,B=0.000000,A=1.000000)")
  (CallFunction|LoadPlayerStats))

(fn ConstructionScript)